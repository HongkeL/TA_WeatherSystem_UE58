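; Dynamic sky actor that sets up time of day, weather, moon, stars and clouds from its construction script, with no runtime logic.
; TimeOfDay rotates and toggles the sun and moon lights, switching lighting between the weather preset by day and moon settings at night.
; A dynamic sky-sphere material drives stars, moon and 2D clouds, alongside optional volumetric clouds.
; Snowy weather forces late morning, hides clouds and flags snow through a material parameter collection.
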(event EventBeginPlay)

(event Collision|EventActorBeginOverlap
  (params (OtherActor :type Actor%20Object%20Reference)))

(event EventTick
  (params (DeltaSeconds :type Float%20%28single-precision%29)))

(fn ConstructionScript
  ;[1 1 1] before call HandleNightSettings, get refrence of MI_DynamicSkySphere
  (bind _is_dynmi_skyspherevalid (01-BasicSettings|InitSkySphereMaterial))
  (if _is_dynmi_skyspherevalid
    (Utilities|FlowControl|Sequence
      (:then_0
        (04_WeatherSettings|HandleWeatherSettings))
      (:then_1
        (01-BasicSettings|HandleSunMoonRotation))
      (:then_2
        (01-BasicSettings|HandleVisibility))
      (:then_3
        (02-NightSettings|HandleNightSettings))
      (:then_4
        (03-CloudSettings|HandleCloudSettings)))))

(fn InitSkySphereMaterial
  ;[1 1 1] Get refence of MI_DynamicSkySphere, and define a variable -- Created_DynMI_SkySphere, and it store this refence.
  (bind _returnvalue (Rendering|Material|CreateDynamicMaterialInstance (Variables|Default|GetSM_SkySphere) 0 "/Game/Materials/Sky/MI_DynamicSkySphere.MI_DynamicSkySphere" "None" :!class /Script/Engine.PrimitiveComponent))
  (bind _output_get (Variables|Default|SetCreated_DynMI_SkySphere _returnvalue))
  (return (Utilities|IsValid _output_get)))

(fn HandleSunMoonRotation
  ;[1 1 1] Handle sun rotation between dawn and dusk
  (Transformation|SetWorldRotation (Variables|Default|GetSunDirectionalLight) (Math|Rotator|MakeRotator 0.0 (Math|Float|MapRangeUnclamped (Variables|01-BasicSettings|GetTimeOfDay) (Variables|01-BasicSettings|GetDawnTime) (Variables|01-BasicSettings|GetDuskTime) 0.0 -1.8e+02) (Variables|01-BasicSettings|GetSunMoonRotation)) false false)
  ;[1 1 1] Handle moon rotation after dusk, in this time, moon rises gradually
  (Transformation|SetWorldRotation (Variables|Default|GetMoonDirectionalLight) (Math|Rotator|MakeRotator 0.0 (Math|Float|MapRangeUnclamped (Variables|01-BasicSettings|GetTimeOfDay) (+ (Variables|01-BasicSettings|GetDuskTime) 0.3) 24.0 0.0 -9e+01) (Variables|01-BasicSettings|GetSunMoonRotation)) false false)
  ;[1 1 1] Handle moon rotation before dawn, in this time,  moon falls gradually
  (Transformation|SetWorldRotation (Variables|Default|GetMoonDirectionalLight) (Math|Rotator|MakeRotator 0.0 (Math|Float|MapRangeUnclamped (Variables|01-BasicSettings|GetTimeOfDay) 0.0 (- (Variables|01-BasicSettings|GetDawnTime) 0.3) -9e+01 -1.8e+02) (Variables|01-BasicSettings|GetSunMoonRotation)) false false))

(fn HandleVisibility
  ;[1 1 1] When it's daytime, only has sun directional light,
  ; When it's nighttime, only has moon directional light.
  (Rendering|SetVisibility (Variables|Default|GetSunDirectionalLight) (Utilities|IsDayTime) false)
  (Rendering|SetVisibility (Variables|Default|GetMoonDirectionalLight) (Utilities|IsNightTime) false))

(fn HandleNightSettings
  (if (Utilities|IsNightTime)
    (Utilities|FlowControl|Sequence
      (:then_0
        ;[1 1 1] Set properties for moon directional light in the nighttime
        (Rendering|Components|Light|SetIntensity (Variables|Default|GetMoonDirectionalLight) (Variables|02-NightSettings|GetMoon%20Light%20Intensity))
        (Rendering|Components|Light|SetLightColor (Variables|Default|GetMoonDirectionalLight) (Variables|02-NightSettings|GetMoon%20Light%20Color) true)
        (Class|DirectionalLightComponent|SetLightSourceAngle (Variables|Default|GetMoonDirectionalLight) (Variables|02-NightSettings|GetMoon%20Light%20Source%20Angle))
        (Class|LightComponent|SetTemperature (Variables|Default|GetMoonDirectionalLight) (Variables|02-NightSettings|GetMoon%20Light%20Temperature)))
      (:then_1
        ;[1 1 1] Set properties for sky atmosphere in the nighttime
        (Class|SkyAtmosphereComponent|SetRayleighScattering (Variables|Default|GetSkyAtmosphere) (Variables|02-NightSettings|GetNighttime%20Rayleigh%20Scattering))
        (Class|SkyAtmosphereComponent|SetMultiScatteringFactor (Variables|Default|GetSkyAtmosphere) (Variables|02-NightSettings|GetNighttime%20Multi%20Cattering)))
      (:then_2
        ;[1 1 1] Modify IsStarVisible when nighttime
        (Rendering|Material|SetScalarParameterValue (Variables|Default|GetCreated_DynMI_SkySphere) "IsStarVisible" (Math|Float|SelectFloat 1.0 0.0 (Variables|02-NightSettings|GetShouldShowStars)) :!class /Script/Engine.MaterialInstanceDynamic)
        ;[1 1 1] Modify IsMoonVisible when nighttime
        (Rendering|Material|SetScalarParameterValue (Variables|Default|GetCreated_DynMI_SkySphere) "IsMoonVisible" (Math|Float|SelectFloat 1.0 0.0 (Variables|02-NightSettings|GetShouldShowMoon)) :!class /Script/Engine.MaterialInstanceDynamic)
        ;[1 1 1] Show the value of MoonSettings and MoonTint in the blueprint details
        (Rendering|Material|SetVectorParameterValue (Variables|Default|GetCreated_DynMI_SkySphere) "MoonSettings" (Utilities|Struct|MakeLinearColor (/ (Variables|02-NightSettings|GetMoonScale) 1e+01) (Variables|02-NightSettings|GetMoonStaticRotation) (Variables|02-NightSettings|GetMoonBrightness) 1.0) :!class /Script/Engine.MaterialInstanceDynamic)
        (Rendering|Material|SetVectorParameterValue (Variables|Default|GetCreated_DynMI_SkySphere) "MoonTint" (Variables|02-NightSettings|GetMoonTint) :!class /Script/Engine.MaterialInstanceDynamic)))
    (else
      (04_WeatherSettings|HandleWeatherSettings)
      ;[1 1 1] Modify IsStarVisible when daytime
      (Rendering|Material|SetScalarParameterValue (Variables|Default|GetCreated_DynMI_SkySphere) "IsStarVisible" 0.0 :!class /Script/Engine.MaterialInstanceDynamic)
      ;[1 1 1] Modify IsMoonVisible when daytime
      (Rendering|Material|SetScalarParameterValue (Variables|Default|GetCreated_DynMI_SkySphere) "IsMoonVisible" 0.0 :!class /Script/Engine.MaterialInstanceDynamic))))

(fn HandleCloudSettings
  (Utilities|GetCurrentWeatherType
    (:Sunny
      ;[1 1 1] If CurrentCloudMode = none, ShouldShow = 0;
      ; If CurrentCloudMode = 2D Cloud, ShouldShow = 1.
      (switch Utilities|FlowControl|Switch|SwitchonECloudMode (Variables|03-CloudSettings|GetCurrentCloudMode)
        (:NewEnumerator0
          (Utilities|Toggle2DClouds false)
          (Utilities|ToggleVolumetricClouds false))
        (:NewEnumerator1
          (Utilities|Toggle2DClouds true)
          (Utilities|Set2DCloudsSettings)
          (Utilities|ToggleVolumetricClouds false))
        (:NewEnumerator2
          (Utilities|Toggle2DClouds false)
          (Utilities|ToggleVolumetricClouds true)
          (Utilities|SetVolumetricCloudSettings))))
    (:Snowy
      (Utilities|Toggle2DClouds false)
      (Utilities|ToggleVolumetricClouds false))))

(fn HandleWeatherSettings
  (04_WeatherSettings|SetWeatherLightingProperties)
  (Utilities|GetCurrentWeatherType
    (:Sunny
      (Utilities|ToggleSnow false))
    (:Snowy
      (Variables|01-BasicSettings|SetTimeOfDay 11.0)
      (Utilities|ToggleSnow true))))

(fn SetWeatherLightingProperties
  (bind _currentweatherpreset (Variables|04_WeatherSettings|GetCurrentWeatherPreset))
  (bind _currentweatherpreset_2 (Variables|04_WeatherSettings|GetCurrentWeatherPreset))
  (bind _currentweatherpreset_3 (Variables|04_WeatherSettings|GetCurrentWeatherPreset))
  (bind _directionallightsettings (Variables|/Game/DataAssets/BP_WeatherDataAssetBase.BP_WeatherDataAssetBase_C|GetDirectionalLightSettings _currentweatherpreset))
  (bind _skyatmospheresettings (Variables|/Game/DataAssets/BP_WeatherDataAssetBase.BP_WeatherDataAssetBase_C|GetSkyAtmosphereSettings _currentweatherpreset_2))
  (bind _exponentailheightfogsettings (Variables|/Game/DataAssets/BP_WeatherDataAssetBase.BP_WeatherDataAssetBase_C|GetExponentailHeightFogSettings _currentweatherpreset_3))
  (bind (_intensity _lightcolor _sourceangle _temperature) (Utilities|Struct|BreakS_DirectionalLightSettings _directionallightsettings))
  (bind (_multiscattering _rayleighscattering _miescatteringscale _mieabsorptionscale _mieanisotropy _aerialperspectiveviewdistancescale) (Utilities|Struct|BreakS_SkyAtmosphereSettings _skyatmospheresettings))
  (bind (_emissivcolor _extinctionscale) (Utilities|Struct|BreakS_ExponentailHeightFogSettings _exponentailheightfogsettings))
  (if (Utilities|IsDayTime)
    (Utilities|FlowControl|Sequence
      (:then_0
        ;[0.15 0.15 0.15 0.5] Set SunDirectionalLight
        (Rendering|Components|Light|SetIntensity (Variables|Default|GetSunDirectionalLight) _intensity)
        (Rendering|Components|Light|SetLightColor (Variables|Default|GetSunDirectionalLight) _lightcolor true)
        (Class|DirectionalLightComponent|SetLightSourceAngle (Variables|Default|GetSunDirectionalLight) _sourceangle)
        (Class|LightComponent|SetTemperature (Variables|Default|GetSunDirectionalLight) _temperature))
      (:then_1
        ;[0.15 0.15 0.15 0.5] Set SkyLight
        (Rendering|Components|Light|SetIntensity (Variables|Default|GetSkyLight) (Utilities|Struct|BreakS_SkyLightSettings (Variables|/Game/DataAssets/BP_WeatherDataAssetBase.BP_WeatherDataAssetBase_C|GetSkyLightSettings (Variables|04_WeatherSettings|GetCurrentWeatherPreset)))))
      (:then_2
        ;[0.15 0.15 0.15 0.5] Set SkyAtmosphere
        (Class|SkyAtmosphereComponent|SetMultiScatteringFactor (Variables|Default|GetSkyAtmosphere) _multiscattering)
        (Class|SkyAtmosphereComponent|SetRayleighScattering (Variables|Default|GetSkyAtmosphere) _rayleighscattering)
        (Class|SkyAtmosphereComponent|SetMieScatteringScale (Variables|Default|GetSkyAtmosphere) _miescatteringscale)
        (Class|SkyAtmosphereComponent|SetMieAbsorptionScale (Variables|Default|GetSkyAtmosphere) _mieabsorptionscale)
        (Class|SkyAtmosphereComponent|SetMieAnisotropy (Variables|Default|GetSkyAtmosphere) _mieanisotropy)
        (Class|SkyAtmosphereComponent|SetAerialPespectiveViewDistanceScale (Variables|Default|GetSkyAtmosphere) _aerialperspectiveviewdistancescale))
      (:then_3
        ;[0.15 0.15 0.15 0.5] Set ExponentialHeightFog
        (Class|ExponentialHeightFogComponent|SetVolumetricFogEmissive (Variables|Default|GetExponentialHeightFog) _emissivcolor)
        (Class|ExponentialHeightFogComponent|SetVolumetricFogExtinctionScale (Variables|Default|GetExponentialHeightFog) _extinctionscale)))))